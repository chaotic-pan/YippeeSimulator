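; BP_Desk is a desk prop with eight small and two big drawers, posed by a Closed flag.
; The Construction Script slides each drawer back along local X by a preset amount when Closed is true, and sets it to zero relative location otherwise.
; The event graph holds only disabled stub events, so the Blueprint adds no runtime interaction or animation.
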(event EventBeginPlay)

(event Collision|EventActorBeginOverlap
  (params (OtherActor :type Actor%20Object%20Reference)))

(event EventTick
  (params (DeltaSeconds :type Float%20%28single-precision%29)))

(fn ConstructionScript
  (if (Variables|Default|Getclosed)
    (LocalVariables|SetPos1 "-7.000000,0.000000,0.000000")
    (LocalVariables|SetPos2 "-9.500000,0.000000,0.000000")
    (LocalVariables|SetPos3 "-12.000000,0.000000,0.000000")
    (LocalVariables|SetPos4 "-16.000000,0.000000,0.000000")
    (LocalVariables|SetPos5 "-12.000000,0.000000,0.000000")
    (LocalVariables|SetPos6 "-17.000000,0.000000,0.000000")
    (LocalVariables|SetPos7 "-20.000000,0.000000,0.000000")
    (LocalVariables|SetPos8 "-24.000000,0.000000,0.000000")
    (LocalVariables|SetPosB1 "-20.000000,0.000000,0.000000")
    (LocalVariables|SetPosB2 "-20.000000,0.000000,0.000000")
    (else
      (LocalVariables|SetPos1 "0, 0, 0")
      (LocalVariables|SetPos2 "0, 0, 0")
      (LocalVariables|SetPos3 "0, 0, 0")
      (LocalVariables|SetPos4 "0, 0, 0")
      (LocalVariables|SetPos5 "0, 0, 0")
      (LocalVariables|SetPos6 "0, 0, 0")
      (LocalVariables|SetPos7 "0, 0, 0")
      (LocalVariables|SetPos8 "0, 0, 0")
      (LocalVariables|SetPosB1 "0, 0, 0")
      (LocalVariables|SetPosB2 "0, 0, 0")))
  (Transformation|SetRelativeLocation (Variables|Default|GetsmallDrawer1) (LocalVariables|GetPos1) false false)
  (Transformation|SetRelativeLocation (Variables|Default|GetsmallDrawer2) (LocalVariables|GetPos2) false false)
  (Transformation|SetRelativeLocation (Variables|Default|GetsmallDrawer3) (LocalVariables|GetPos3) false false)
  (Transformation|SetRelativeLocation (Variables|Default|GetsmallDrawer4) (LocalVariables|GetPos4) false false)
  (Transformation|SetRelativeLocation (Variables|Default|GetsmallDrawer5) (LocalVariables|GetPos5) false false)
  (Transformation|SetRelativeLocation (Variables|Default|GetsmallDrawer6) (LocalVariables|GetPos6) false false)
  (Transformation|SetRelativeLocation (Variables|Default|GetsmallDrawer7) (LocalVariables|GetPos7) false false)
  (Transformation|SetRelativeLocation (Variables|Default|GetsmallDrawer8) (LocalVariables|GetPos8) false false)
  (Transformation|SetRelativeLocation (Variables|Default|GetbigDrawer1) (LocalVariables|GetPosB1) false false)
  (Transformation|SetRelativeLocation (Variables|Default|GetbigDrawer2) (LocalVariables|GetPosB2) false false))